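; BP_Powerup_Speed is a speed powerup that temporarily boosts the player pawn's walk speed.
; On activation it hides its mesh, doubles MaxWalkSpeed and plays a scale-up sound.
; On expiry it halves the speed, destroys itself and plays a power-down sound.
; Both changes derive from GetMaxSpeed at that moment rather than a stored original, and timing is not handled in this graph.
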(event EventBeginPlay)

(event Collision|EventActorBeginOverlap
  (params (OtherActor :type Actor%20Object%20Reference)))

(event EventTick
  (params (DeltaSeconds :type Float%20%28single-precision%29)))

(event EventOnExpired
  (bind _returnvalue (Game|Player|GetPlayerPawn 0))
  (bind _returnvalue_2 (Actor|GetComponentbyClass _returnvalue "/Script/Engine.CharacterMovementComponent"))
  (Variables|/Script/Engine.CharacterMovementComponent|SetMaxWalkSpeed _returnvalue_2 (/ (Class|MovementComponent|GetMaxSpeed _returnvalue_2) 2.0))
  (Actor|DestroyActor)
  (Audio|PlaySound2D "/Game/Powerups/powerdown_01.powerdown_01" 1.0 1.0 0.0 0 0))

(event EventOnActivated
  (bind _returnvalue (Game|Player|GetPlayerPawn 0))
  (bind _returnvalue_2 (Actor|GetComponentbyClass _returnvalue "/Script/Engine.CharacterMovementComponent"))
  (Rendering|SetVisibility (Variables|Default|GetStaticMesh) false true)
  (Variables|/Script/Engine.CharacterMovementComponent|SetMaxWalkSpeed _returnvalue_2 (* (Class|MovementComponent|GetMaxSpeed _returnvalue_2) 2.0))
  (Audio|PlaySound2D "/Engine/VREditor/Sounds/UI/Scaling_Up.Scaling_Up" 1.5 1.0 0.0 0 0))

(fn ConstructionScript)