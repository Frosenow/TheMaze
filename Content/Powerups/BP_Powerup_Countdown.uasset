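; BP_Powerup_Countdown is a timer powerup that applies a time amount to the player character's TimerPowerup when activated.
; Activation hides the mesh, calls TimerPowerup on the CFPSCharacter, then shows a WBP_PowerupCountdownText widget with a pop-up animation and plays a 2D sound.
; The sound and widget depend on sequence order rather than the cast, and the actor destroys itself on expiry.
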(event EventOnExpired
  (Actor|DestroyActor))

(event EventOnActivated
  (Utilities|FlowControl|Sequence
    (:then_0
      (Rendering|SetVisibility (Variables|Default|GetStaticMesh) false true))
    (:then_1
      (bind _ascfpscharacter (Utilities|Casting|CastToCFPSCharacter (Game|GetPlayerCharacter 0)))
      (Class|CFPSCharacter|TimerPowerup _ascfpscharacter (Variables|Default|GetTime%20Amount_0)))
    (:then_2
      (bind _returnvalue (UserInterface|CreateWidget "/Game/Blueprints/WBP_PowerupCountdownText.WBP_PowerupCountdownText_C" 0 self))
      (UserInterface|Viewport|AddtoViewport _returnvalue 0)
      (UserInterface|Animation|PlayAnimation _returnvalue (Variables|/Game/Blueprints/WBP_PowerupCountdownText.WBP_PowerupCountdownText_C|GetPopUpAnimation _returnvalue) 1.0 1 "Forward" 0.5 false)
      (Audio|PlaySound2D "/Engine/VREditor/Sounds/UI/Scaling_Up.Scaling_Up" 1.5 1.5 0.0 0 0))))

(fn ConstructionScript)